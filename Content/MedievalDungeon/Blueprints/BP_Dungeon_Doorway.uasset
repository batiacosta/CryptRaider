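; Double-door dungeon doorway actor that wires trigger components to rotator movers for its left and right large door meshes.
; On BeginPlay, each of the two trigger components receives its own rotator mover, and each mover receives its matching door mesh.
; The Blueprint only does this setup, leaving trigger detection and rotation to the components, with no active overlap, Tick or construction logic.
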(event EventBeginPlay
  (Class|TriggerComponent|SetMover (Variables|Default|GetTriggerComponent1) (Variables|Default|GetRotatorIMoverRight))
  (Class|TriggerComponent|SetMover (Variables|Default|GetTriggerComponent2) (Variables|Default|GetRotatorIMoverLeft))
  (Class|RotatorIMover|SetDoorMesh (Variables|Default|GetRotatorIMoverRight) (Variables|Default|GetSM_DoorWay_Large_Door_Right))
  (Class|RotatorIMover|SetDoorMesh (Variables|Default|GetRotatorIMoverLeft) (Variables|Default|GetSM_DoorWay_Large_Door_Left)))

(event Collision|EventActorBeginOverlap
  (params (OtherActor :type Actor%20Object%20Reference)))

(event EventTick
  (params (DeltaSeconds :type Float%20%28single-precision%29)))

(fn ConstructionScript)